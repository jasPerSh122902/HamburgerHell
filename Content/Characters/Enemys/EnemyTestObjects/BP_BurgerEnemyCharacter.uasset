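; BP_BurgerEnemyCharacter is a burger enemy that damages the first-person player on contact and shatters when killed.
; Hitbox overlap with the player applies damage immediately and starts a half-second looping damage timer, cleared when the overlap ends.
; Bullet or missile overlaps check whether health is depleted, then swap the mesh for a destructible one, disable the hitbox and destroy the actor after a short delay.
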(event `self.Hitbox.OnComponentBeginOverlap`
  (params (OverlappedComponent :type "PrimitiveComponent Object Reference") (OtherActor :type "Actor Object Reference") (OtherComp :type "PrimitiveComponent Object Reference") (OtherBodyIndex :type Integer) (bFromSweep :type Boolean) (SweepResult :type "HitResult Structure (by ref)"))
  ;[1 1 1] IsOverlapped is set to true when enemy and player are overlapped
  (bind _asfirst_person_character (cast `/Game/FirstPersonCPP/Blueprints/FirstPersonCharacter` OtherActor))
  (set `self.As First Person Character` _asfirst_person_character)
  (`self.Timer`))

(event `self.Hitbox.OnComponentEndOverlap`
  (params (OverlappedComponent :type "PrimitiveComponent Object Reference") (OtherActor :type "Actor Object Reference") (OtherComp :type "PrimitiveComponent Object Reference") (OtherBodyIndex :type Integer))
  ;[1 1 1] IsOverlapped is set to false when enemy and player are no longer overlapped
  (cast `/Game/FirstPersonCPP/Blueprints/FirstPersonCharacter` OtherActor)
  (`self.ClearTimer`)
  (`self.ClearTimer`))

(event `Timer`
  ;[1 1 1] When player and enemy are overlapped enemy will apply damage and the set a timer to damage palyer
  (`GameplayStatics.ApplyDamage` (`self.As First Person Character`) (`self.m_damage`))
  (`KismetSystemLibrary.K2_SetTimerDelegate` (delegate `DamagePlayer`) 0.5 true) ; DamagePlayer will loop as long as the player and enemy are overlapped
)

(event `DamagePlayer`
  ;[1 1 1] Damage player and spawn player hit indicator
  (`GameplayStatics.ApplyDamage` (`self.As First Person Character`) (`self.m_damage`)))

(event `ClearTimer`
  ;[1 1 1] Stops the timer that loops through DamagePlayer
  (`KismetSystemLibrary.K2_ClearTimer` null "DamagePlayer"))

(event `BulletCollision`
  (params (OtherActor :type "Actor Object Reference"))
  (bind _mesh (`self.Mesh`))
  ;[1 1 1] Activates the destructible mesh and deletes the actor when hp is zero
  (cast `BulletActor` OtherActor)
  (if (<= (`self.m_health`) 0.0)
    (`/Engine/EditorBlueprintResources/StandardMacros.IsValid` _mesh
      (:`Is Valid`
        (`ActorComponent.K2_DestroyComponent` _mesh)
        (`DestructibleComponent.SetDestructibleMesh` (`self.DestructableMesh`) (`self.CurrentDMesh`))
        (`PrimitiveComponent.SetCollisionEnabled` (`self.Hitbox`) "NoCollision")
        (`KismetSystemLibrary.Delay` 1.0)
        (`self.K2_DestroyActor`)))))

(event `MissileCollision`
  (params (OtherActor :type "Actor Object Reference"))
  (bind _mesh (`self.Mesh`))
  ;[1 1 1] Activates the destructible mesh and deletes the actor when hp is zero
  (cast `MissleActor` OtherActor)
  (if (<= (`self.m_health`) 0.0)
    (`/Engine/EditorBlueprintResources/StandardMacros.IsValid` _mesh
      (:`Is Valid`
        (`ActorComponent.K2_DestroyComponent` _mesh)
        (`DestructibleComponent.SetDestructibleMesh` (`self.DestructableMesh`) (`self.CurrentDMesh`))
        (`PrimitiveComponent.SetCollisionEnabled` (`self.Hitbox`) "NoCollision")
        (`KismetSystemLibrary.Delay` 1.0)
        (`self.K2_DestroyActor`)))))

(event `self.ReceiveActorBeginOverlap`
  (params (OtherActor :type "Actor Object Reference"))
  ;[1 1 1] When enemy burger is shot the mesh component is destroyed and the destructible mesh is set
  (`self.MissileCollision` OtherActor)
  (`self.BulletCollision` OtherActor))

(fn `UserConstructionScript`)