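; AI controller for a jumping test enemy that runs the BT_JumpingEnemyTree behavior tree.
; One second after starting the tree, it stores the first player's pawn in the Blackboard's "Enemy" key.
; GetNextDestination rebuilds a spline from supplied world-space points and returns the location one jump distance along it, using the spline to measure distance along a path.
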(event `self.ReceiveBeginPlay`
  (`self.RunBehaviorTree` "/Game/Characters/Enemys/EnemyTestObjects/AI/BT_JumpingEnemyTree.BT_JumpingEnemyTree")
  (`KismetSystemLibrary.Delay` 1.0)
  (`BlackboardComponent.SetValueAsObject` (`self.Blackboard`) "Enemy" (`GameplayStatics.GetPlayerPawn` 0)))

(fn `GetNextDestination`
  (params (Points :type "Array of Vector Structure") (JumpDistance :type "Float (double-precision)"))
  (returns (ReturnValue :type "Vector Structure"))
  (`SplineComponent.ClearSplinePoints` (`self.PathSplineComp`) true)
  (`SplineComponent.SetSplinePoints` (`self.PathSplineComp`) Points "World" true)
  (return (`SplineComponent.GetLocationAtDistanceAlongSpline` (`self.PathSplineComp`) JumpDistance "World")))

(fn `UserConstructionScript`)